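; Mystery ship actor that flies along the world X axis with looping or one-shot audio and can be shot down by projectiles.
; A Movement timeline drives SetPosition, adding a swept offset from speed, forward-vector X sign and timeline alpha each update.
; Halt and Resume pause and continue movement and audio.
; Hit fires OnMysteryShipHit, plays a sound at the game instance's SFX volume, hides the ship and destroys it after a short delay.
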(event Custom|StartMovement
  ;[1 1 1] Move
  (bind _alpha (Timeline|Movement PlayFromStart)
    (:Update
      (CallFunction|SetPosition _alpha))))

(event Custom|StopMovement
  ;[1 1 1] Move
  (bind _alpha (Timeline|Movement Stop)
    (:Update
      (CallFunction|SetPosition _alpha))))

(event Custom|Halt
  ;[1 1 1] Halt
  (CallFunction|StopMovement)
  (Class|AudioComponent|SetPaused (Variables|Default|GetAudio) true))

(event Custom|Resume
  ;[1 1 1] Resume
  (CallFunction|ContinueMovement)
  (Class|AudioComponent|SetPaused (Variables|Default|GetAudio) false))

(event Custom|ContinueMovement
  ;[1 1 1] Move
  (bind _alpha (Timeline|Movement Play)
    (:Update
      (CallFunction|SetPosition _alpha))))

(event EventBeginPlay
  ;[1 1 1] Initialise
  (CallFunction|SetReferences)
  (CallFunction|SetAudioComponentVolumeMultiplier)
  (CallFunction|StartMovement))

(event EventHit
  ;[1 1 1] Mystery Ship Hit by Projectile
  (Default|CallOnMysteryShipHit)
  (Audio|PlaySound2D "/Game/Audio/MysteryShipDestroyed_Cue.MysteryShipDestroyed_Cue" (Variables|/Game/SI_GameInstance.SI_GameInstance_C|GetSFXVolumeMultiplier (Variables|Default|GetGameInstanceReference)) 1.0 0.0 0 0)
  (Rendering|SetActorHiddenInGame true)
  (Collision|SetCollisionEnabled (Variables|Default|GetCollision) "NoCollision")
  (Utilities|FlowControl|Delay 0.25)
  (Actor|DestroyActor))

(fn ConstructionScript)

(fn SetPosition
  (params (Alpha :type Float%20%28single-precision%29))
  ;[1 1 1] Set Position
  (Transformation|SetActorLocation (+ (Transformation|GetActorLocation) (* (Math|Vector|MakeVector (* (Variables|Movement|GetMovementSpeed) (.x (Math|Vector|Normalize (Transformation|GetActorForwardVector)))) 0.0 0.0) Alpha)) true false))

(fn SetReferences
  ;[1 1 1] Set References
  (bind _assi_game_instance (Utilities|Casting|CastToSI_GameInstance (Game|GetGameInstance)))
  (Variables|Default|SetGameInstanceReference _assi_game_instance))

(fn SetAudioComponentVolumeMultiplier
  ;[1 1 1] Set Audio Component Volume Multiplier
  (Audio|Components|Audio|SetVolumeMultiplier (Variables|Default|GetAudio) (Variables|/Game/SI_GameInstance.SI_GameInstance_C|GetSFXVolumeMultiplier (Variables|Default|GetGameInstanceReference)) :!class /Script/Engine.AudioComponent))