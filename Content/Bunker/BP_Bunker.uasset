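; Destructible bunker made of BP_BunkerBlock child actors, playing a sound when hit by a projectile or invader unless one is already playing.
; On BeginPlay it caches the game instance, applies SFX volume, collects its blocks and binds to their destroyed events.
; When remaining blocks fall to the game instance's threshold, it self-destructs, exploding them one by one with a delay, then broadcasts OnSelfDestructed and destroys itself.
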(event Custom|SelfDestruct
  ;[1 1 1] Self Destruct
  (Variables|Default|SetIsSelfDestructing true)
  (bind _arrayelement (Utilities|ForEachLoopwithDelay (Variables|Default|GetBunkerBlocks) (Variables|/Game/SI_GameInstance.SI_GameInstance_C|GetBunkerSelfDestructBlockDelay (Variables|Default|GetGameInstanceReference)))
    (:LoopBody
      (Utilities|IsValid _arrayelement
        (:Is%20Valid
          (Effects|SpawnEmitteratLocation "/Game/Assets/Particles/P_Pixel_Explosion.P_Pixel_Explosion" (Transformation|GetActorLocation _arrayelement) "0.000000, 0, 0")
          (Actor|DestroyActor _arrayelement))))
    (:Completed
      (Default|CallOnSelfDestructed self)
      (Actor|DestroyActor))))

(event EventBeginPlay
  ;[1 1 1] Initialise
  (CallFunction|SetReferences)
  (CallFunction|SetAudioComponentVolumeMultiplier)
  (CallFunction|CastChildActors)
  (CallFunction|BindtoBunkerBlockEvents))

(event EventHit
  (params (OtherActor :type Actor%20Object%20Reference))
  ;[1 1 1] Bunker Hit by Projectile or Invader
  (if (not (Audio|Components|Audio|IsPlaying (Variables|Default|GetAudio)))
    (Audio|Components|Audio|Play (Variables|Default|GetAudio) 0.0)))

(fn ConstructionScript)

(fn SetReferences
  ;[1 1 1] Set References
  (bind _assi_game_instance (Utilities|Casting|CastToSI_GameInstance (Game|GetGameInstance)))
  (Variables|Default|SetGameInstanceReference _assi_game_instance))

(fn SetAudioComponentVolumeMultiplier
  ;[1 1 1] Set Audio Component Volume Multiplier
  (Audio|Components|Audio|SetVolumeMultiplier (Variables|Default|GetAudio) (Variables|/Game/SI_GameInstance.SI_GameInstance_C|GetSFXVolumeMultiplier (Variables|Default|GetGameInstanceReference)) :!class /Script/Engine.AudioComponent))

(fn BindtoBunkerBlockEvents
  ;[1 1 1] Bind to Bunker Block Events
  (for _array_element (Variables|Default|GetBunkerBlocks)
    (EventDispatchers|BindEventtoOnBunkerBlockDestroyed _array_element (EventDispatchers|CreateEvent :!event BunkerBlockDestroyed))))

(fn BunkerBlockDestroyed
  (params (BunkerBlock :type BP%20Bunker%20Block%20Object%20Reference))
  ;[1 1 1] Bunker Block Destroyed
  (Utilities|Array|RemoveItem (Variables|Default|GetBunkerBlocks) BunkerBlock)
  (if (and (<= (Utilities|Array|Length (Variables|Default|GetBunkerBlocks)) (Variables|/Game/SI_GameInstance.SI_GameInstance_C|GetBunkerSelfDestructThreshold (Variables|Default|GetGameInstanceReference))) (Math|Boolean|NotEqual(Boolean) (Variables|Default|GetIsSelfDestructing) true))
    (Variables|Default|SetIsSelfDestructing true)
    (CallFunction|SelfDestruct)))

(fn CastChildActors
  ;[1 1 1] Cast Child Actors
  (for _array_element (Actor|GetAllChildActors true)
    (bind _asbp_bunker_block (Utilities|Casting|CastToBP_BunkerBlock _array_element))
    (Utilities|Array|Add (Variables|Default|GetBunkerBlocks) _asbp_bunker_block)))