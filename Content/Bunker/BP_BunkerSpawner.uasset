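; BP_BunkerSpawner spawns BP_Bunker actors at locations stored in the SI_GameInstance, one after another with a delay between each.
; On BeginPlay it caches the game instance and computes TotalSpawnDelay from the location count times the per-bunker delay.
; The SpawnBunkers event loops through the locations with a delayed ForEach, spawning each bunker unrotated at unit scale, regardless of collision.
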(event Custom|SpawnBunkers
  (bind _gameinstancereference (Variables|References|GetGameInstanceReference))
  ;[1 1 1] Spawn Bunkers
  (bind _arrayelement (Utilities|ForEachLoopwithDelay (Variables|/Game/SI_GameInstance.SI_GameInstance_C|GetBunkerSpawnLocations _gameinstancereference) (Variables|/Game/SI_GameInstance.SI_GameInstance_C|GetBunkerSpawnDelay _gameinstancereference))
    (:LoopBody
      (bind _spawntransform (CallFunction|GetSpawnTransform _arrayelement))
      (Game|SpawnActorfromClass "/Game/Bunker/BP_Bunker.BP_Bunker_C" _spawntransform "AlwaysSpawn" 0 0))))

(event EventBeginPlay
  ;[1 1 1] Initialise
  (CallFunction|CreateReferences)
  (CallFunction|SetTotalSpawnDelay))

(fn ConstructionScript)

(fn GetSpawnTransform
  (params (SpawnLocation :type Vector))
  ;[1 1 1] Get Spawn Transform
  (return (Math|Transform|MakeTransform SpawnLocation)))

(fn CreateReferences
  ;[1 1 1] Create References
  (bind _assi_game_instance (Utilities|Casting|CastToSI_GameInstance (Game|GetGameInstance)))
  (Variables|References|SetGameInstanceReference _assi_game_instance))

(fn SetTotalSpawnDelay
  (bind _gameinstancereference (Variables|References|GetGameInstanceReference))
  ;[1 1 1] Set Total Spawn Delay
  (Variables|Default|SetTotalSpawnDelay (* (Utilities|Array|Length (Variables|/Game/SI_GameInstance.SI_GameInstance_C|GetBunkerSpawnLocations _gameinstancereference)) (Variables|/Game/SI_GameInstance.SI_GameInstance_C|GetBunkerSpawnDelay _gameinstancereference))))