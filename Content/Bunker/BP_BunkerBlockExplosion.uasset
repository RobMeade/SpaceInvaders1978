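; BP_BunkerBlockExplosion is the explosion actor for bunker blocks, carrying a sphere component that defines its radius.
; On BeginPlay it caches the SI_GameInstance, then sets the ExplosionRadius sphere size from the game instance's BunkerBlockExplosionRadius value.
; The radius is set without updating overlaps, and the file contains no damage, effect or destruction logic.
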(event EventBeginPlay
  ;[1 1 1] Initialise
  (CallFunction|SetReferences)
  (CallFunction|ConfigureExplosion))

(fn ConstructionScript)

(fn SetReferences
  ;[1 1 1] Set References
  (bind _assi_game_instance (Utilities|Casting|CastToSI_GameInstance (Game|GetGameInstance)))
  (Variables|References|SetGameInstanceReference _assi_game_instance))

(fn ConfigureExplosion
  ;[1 1 1] Configure Explosion
  (Components|Sphere|SetSphereRadius (Variables|Default|GetExplosionRadius) (Variables|/Game/SI_GameInstance.SI_GameInstance_C|GetBunkerBlockExplosionRadius (Variables|References|GetGameInstanceReference)) false))