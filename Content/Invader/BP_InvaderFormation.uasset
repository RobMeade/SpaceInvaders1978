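; Space Invaders-style formation actor that spawns a grid of invaders, typed by row and attached to it, then moves and attacks with them as one body.
; A timeline sweeps it sideways; collision bounds fitted to surviving invaders trigger descent and reversal, or game over on one specific channel.
; Another timeline fires from random invaders, one projectile at a time.
; Clearing the formation resets its position and revives attached invaders before attacking again.
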(event OnComponentBeginOverlap(Collision)
  (params (OverlappedComponent :type Primitive%20Component%20Object%20Reference) (OtherActor :type Actor%20Object%20Reference) (OtherComp :type Primitive%20Component%20Object%20Reference) (OtherBodyIndex :type Integer) (bFromSweep :type Boolean) (SweepResult :type Hit%20Result%20Structure%20%28by%20ref%29))
  ;[1 1 1] Boundary Collision
  (if (Variables|InvaderFormation|Movement|GetMovementEnabled)
    (if (Utilities|Enum|Equal(Enum) (Collision|GetCollisionObjectType OtherComp) "ECC_GameTraceChannel2")
      (CallFunction|HaltAttack)
      (Default|GameOver (Variables|References|GetGameModeReference))
      (else
        (CallFunction|Descend)
        (CallFunction|ReverseDirection)))))

(event Custom|OnInvaderProjectileDestroyed
  ;[1 1 1] Firing
  (Variables|InvaderFormation|Firing|SetCanFire true)
  (Variables|InvaderFormation|Spawn|SetCanRespawn true))

(event Custom|BeginAttack
  ;[1 1 1] Begin Attack
  (CallFunction|ResetPosition)
  (Variables|InvaderFormation|Movement|SetMovementRight true)
  (Variables|InvaderFormation|Movement|SetMovementEnabled true)
  (CallFunction|Move)
  (Variables|InvaderFormation|Firing|SetFiringEnabled true)
  (Variables|InvaderFormation|Firing|SetCanFire true)
  (CallFunction|Fire))

(event Custom|Respawn
  ;[1 1 1] Respawn
  (CallFunction|ResetPosition)
  (for _array_element (Actor|GetAttachedActors)
    (bind _asbp_invader_base (Utilities|Casting|CastToBP_Invader_Base _array_element))
    (Utilities|Array|Add (Variables|InvaderFormation||GetInvaders) _asbp_invader_base)
    (for _array_element_2 (Variables|InvaderFormation||GetInvaders)
      (Rendering|SetActorHiddenInGame _array_element_2 false)
      (Collision|SetCollisionEnabled (Variables|/Game/Invader/BP_Invader_Base.BP_Invader_Base_C|GetCollision _array_element_2) "QueryOnly"))
    (CallFunction|UpdateCollisionVolumeExtentsandPosition)
    (Utilities|FlowControl|Delay 1.0)
    (while (Math|Boolean|NotEqual(Boolean) (Variables|InvaderFormation|Spawn|GetCanRespawn) true)
      _)
    (CallFunction|BeginAttack)))

(event Custom|Move
  ;[1 1 1] Movement
  (bind _alpha (Timeline|Movement PlayFromStart)
    (:Update
      (if (Variables|InvaderFormation|Movement|GetMovementEnabled)
        (CallFunction|SetPosition _alpha)
        (else
          (CallFunction|StopMoving))))))

(event Custom|Descend
  ;[1 1 1] Descend
  (bind _descentlocation (CallFunction|GetDescentPosition))
  (Transformation|SetActorLocation _descentlocation true false))

(event Custom|StopMoving
  ;[1 1 1] Movement
  (bind _alpha (Timeline|Movement Stop)
    (:Update
      (if (Variables|InvaderFormation|Movement|GetMovementEnabled)
        (CallFunction|SetPosition _alpha)
        (else
          (CallFunction|StopMoving))))))

(event Custom|ReverseDirection
  ;[1 1 1] Reverse Direction
  (Variables|InvaderFormation|Movement|SetMovementRight (not (Variables|InvaderFormation|Movement|GetMovementRight))))

(event Custom|HaltAttack
  ;[1 1 1] Halt Attack
  (Variables|InvaderFormation|Movement|SetMovementEnabled false)
  (CallFunction|StopMoving)
  (Variables|InvaderFormation|Firing|SetFiringEnabled false)
  (CallFunction|StopFiring))

(event Custom|Fire
  ;[1 1 1] Firing
  (Timeline|Firing PlayFromStart
    (:Update
      (if (Variables|InvaderFormation|Firing|GetFiringEnabled)
        (if (Variables|InvaderFormation|Firing|GetCanFire)
          (bind _invader (CallFunction|GetRandomInvader))
          (Utilities|IsValid _invader
            (:Is%20Valid
              (EventDispatchers|BindEventtoOnProjectileDestroyed _invader (delegate Custom|OnInvaderProjectileDestroyed))
              (Default|Fire _invader)
              (Variables|InvaderFormation|Firing|SetCanFire false)
              (Variables|InvaderFormation|Spawn|SetCanRespawn false))))
        (else
          (CallFunction|StopFiring))))))

(event Custom|ResumeAttack
  ;[1 1 1] Resume Attack
  (Variables|InvaderFormation|Movement|SetMovementEnabled true)
  (CallFunction|Move)
  (Variables|InvaderFormation|Firing|SetFiringEnabled true)
  (CallFunction|Fire))

(event Custom|StopFiring
  ;[1 1 1] Firing
  (Timeline|Firing Stop
    (:Update
      (if (Variables|InvaderFormation|Firing|GetFiringEnabled)
        (if (Variables|InvaderFormation|Firing|GetCanFire)
          (bind _invader (CallFunction|GetRandomInvader))
          (Utilities|IsValid _invader
            (:Is%20Valid
              (EventDispatchers|BindEventtoOnProjectileDestroyed _invader (delegate Custom|OnInvaderProjectileDestroyed))
              (Default|Fire _invader)
              (Variables|InvaderFormation|Firing|SetCanFire false)
              (Variables|InvaderFormation|Spawn|SetCanRespawn false))))
        (else
          (CallFunction|StopFiring))))))

(event EventBeginPlay
  ;[1 1 1] Initialise
  (CallFunction|SetReferences)
  (CallFunction|SetStructure)
  (CallFunction|Spawn))

(fn ConstructionScript)

(fn SetStructure
  ;[1 1 1] Set Structure
  (Variables|InvaderFormation|Spawn|SetRows 5)
  (Variables|InvaderFormation|Spawn|SetColumns 11))

(fn Spawn
  ;[1 1 1] Spawn
  (for _index (range 0 (- (Variables|InvaderFormation|Spawn|GetRows) 1))
    (bind _invadertype (CallFunction|GetInvaderTypebyRowIndex _index))
    (for _index_2 (range 0 (- (Variables|InvaderFormation|Spawn|GetColumns) 1))
      (bind _invader (CallFunction|SpawnInvader _invadertype))
      (CallFunction|SetSpawnedInvaderPosition _invader _index_2 _index)
      (Transformation|AttachActorToActor _invader self "None" "KeepRelative" "KeepRelative" "KeepRelative" true)
      (CallFunction|UpdateCollisionVolumeExtentsandPosition))))

(fn SpawnInvader
  (params (InvaderType :type E_InvaderType%20Enum :default "NewEnumerator0"))
  ;[1 1 1] Spawn Invader
  (bind _invaderclass (CallFunction|GetInvaderClassbyType InvaderType))
  (bind _returnvalue (Game|SpawnActorfromClass _invaderclass (Transformation|GetActorTransform) "AlwaysSpawn" 0 0))
  (bind _output_get (LocalVariables|SetSpawnedInvader _returnvalue))
  (CallFunction|BindtoInvaderEvents _output_get)
  (Utilities|FlowControl|Sequence
    (:then_0
      (Utilities|FlowControl|DoOnce false
        (:Completed
          (Variables|InvaderFormation|Spawn|SetSpawnPositionOffset (Components|Box|GetUnscaledBoxExtent (Variables|/Game/Invader/BP_Invader_Base.BP_Invader_Base_C|GetCollision (LocalVariables|GetSpawnedInvader)))))))
    (:then_1
      (Utilities|Array|Add (Variables|InvaderFormation||GetInvaders) (LocalVariables|GetSpawnedInvader))
      (return (LocalVariables|GetSpawnedInvader)))))

(fn SetSpawnedInvaderPosition
  (params (Invader :type BP%20Invader%20Base%20Object%20Reference) (Column :type Integer) (Row :type Integer))
  ;[1 1 1] Set Invader Position
  (Transformation|SetActorTransform Invader (Math|Transform|MakeTransform (* (Math|Vector|MakeVector (* Column (.x (Variables|InvaderFormation|Spawn|GetSpawnPositionOffset))) 0.0 (* (* Row (.z (Variables|InvaderFormation|Spawn|GetSpawnPositionOffset))) -1.0)) 2)))
  (return))

(fn UpdateCollisionVolumeExtentsandPosition
  ;[1 1 1] Update Collision Volume Extents and Positions
  (bind (_center _boxextent) (Collision|GetActorArrayBounds (Variables|InvaderFormation||GetInvaders)))
  (Components|Box|SetBoxExtent (Variables|Default|GetCollision) _boxextent true)
  (if (> (Utilities|Array|Length (Variables|InvaderFormation||GetInvaders)) 0)
    (Transformation|SetWorldLocation (Variables|Default|GetCollision) _center false false)))

(fn SetReferences
  ;[1 1 1] Set References
  (bind _assi_game_instance (Utilities|Casting|CastToSI_GameInstance (Game|GetGameInstance)))
  (Variables|References|SetGameInstanceReference _assi_game_instance)
  (bind _assi_game_mode_base (Utilities|Casting|CastToSI_GameMode_Base (Game|GetGameMode)))
  (Variables|References|SetGameModeReference _assi_game_mode_base))

(fn ResetPosition
  ;[1 1 1] Reset Invader Formation Position
  (Transformation|SetActorLocation (Variables|/Game/SI_GameInstance.SI_GameInstance_C|GetInvaderFormationSpawnLocation (Variables|References|GetGameInstanceReference)) false false))

(fn GetDescentPosition
  (bind _returnvalue (Transformation|GetActorLocation))
  ;[1 1 1] Get Descent Position
  (return (Math|Vector|MakeVector (.x _returnvalue) 0.0 (- (.z _returnvalue) (* (.z (Variables|InvaderFormation|Spawn|GetSpawnPositionOffset)) (Variables|InvaderFormation|Movement|GetDescentMultiplier))))))

(fn SetPosition
  (params (Alpha :type Float%20%28single-precision%29))
  ;[1 1 1] Set Position
  (Transformation|SetActorLocation (+ (Transformation|GetActorLocation) (* (Math|Vector|MakeVector (* (Variables|InvaderFormation|Movement|GetMovementSpeed) (Math|Float|SelectFloat 1.0 -1.0 (Variables|InvaderFormation|Movement|GetMovementRight))) 0.0 0.0) Alpha)) true false))

(fn BindtoInvaderEvents
  (params (Invader :type BP%20Invader%20Base%20Object%20Reference))
  ;[1 1 1] Bind to Invader Events
  (EventDispatchers|BindEventtoOnInvaderDestroyed Invader (EventDispatchers|CreateEvent :!event InvaderDestroyed)))

(fn InvaderDestroyed
  (params (Invader :type BP%20Invader%20Base%20Object%20Reference))
  ;[1 1 1] OnInvaderDestroyed
  (Utilities|Array|RemoveItem (Variables|InvaderFormation||GetInvaders) Invader)
  (CallFunction|UpdateCollisionVolumeExtentsandPosition)
  (Default|CallOnInvaderDestroyed Invader)
  (if (<= (Utilities|Array|Length (Variables|InvaderFormation||GetInvaders)) 0)
    (Variables|InvaderFormation|Movement|SetMovementEnabled false)
    (Variables|InvaderFormation|Firing|SetFiringEnabled false)
    (CallFunction|Respawn)))

(fn GetInvaderClassbyType
  (params (InvaderType :type E_InvaderType%20Enum :default "NewEnumerator0"))
  ;[1 1 1] Get Invader Class by Type
  (switch Utilities|FlowControl|Switch|SwitchonE_InvaderType InvaderType
    (:NewEnumerator0
      (return "/Game/Invader/BP_Invader1_Child.BP_Invader1_Child_C"))
    (:NewEnumerator1
      (return "/Game/Invader/BP_Invader2_Child.BP_Invader2_Child_C"))
    (:NewEnumerator2
      (return "/Game/Invader/BP_Invader3_Child.BP_Invader3_Child_C"))))

(fn GetInvaderTypebyRowIndex
  (params (Index :type Integer))
  ;[1 1 1] Get Invader Type by Row Index
  (if (== Index 0)
    (return "NewEnumerator0")
    (elif (Math|Integer|InRange(Integer) Index 1 2)
      (return "NewEnumerator1")
      (elif (Math|Integer|InRange(Integer) Index 3 4)
        (return "NewEnumerator2")))))

(fn GetRandomInvader
  (bind _invaders (Variables|InvaderFormation||GetInvaders))
  ;[1 1 1] Get Random Invader
  (return (Utilities|Array|Get(acopy) _invaders (Math|Random|RandomIntegerinRange 0 (- (Utilities|Array|Length _invaders) 1)))))