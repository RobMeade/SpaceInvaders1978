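; Base invader actor for a Space Invaders-style game that reacts to being hit.
; An overlap with a component on a custom collision channel destroys the other actor, triggers self-destruct and calls OnInvaderDestroyed with itself.
; Self-destruct hides the invader and disables its collision rather than destroying the actor.
; On BeginPlay it caches a reference to the SI_GameMode.
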(event OnComponentBeginOverlap(Collision)
  (params (OverlappedComponent :type Primitive%20Component%20Object%20Reference) (OtherActor :type Actor%20Object%20Reference) (OtherComp :type Primitive%20Component%20Object%20Reference) (OtherBodyIndex :type Integer) (bFromSweep :type Boolean) (SweepResult :type Hit%20Result%20Structure%20%28by%20ref%29))
  ;[1 1 1] Collision
  (if (Utilities|Enum|Equal(Enum) (Collision|GetCollisionObjectType OtherComp) "ECC_GameTraceChannel1")
    (Actor|DestroyActor OtherActor)
    (CallFunction|SelfDestruct)
    (Default|CallOnInvaderDestroyed self)))

(event Custom|SelfDestruct
  ;[1 1 1] Self Destruct
  (Rendering|SetActorHiddenInGame true)
  (Collision|SetCollisionEnabled (Variables|Default|GetCollision) "NoCollision"))

(event EventBeginPlay
  ;[1 1 1] Initialise
  (CallFunction|SetReferences))

(fn ConstructionScript)

(fn SetReferences
  ;[1 1 1] Set References
  (bind _assi_game_mode (Utilities|Casting|CastToSI_GameMode (Game|GetGameMode)))
  (Variables|Default|SetGameModeReference _assi_game_mode))