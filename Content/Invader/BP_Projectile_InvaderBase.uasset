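; Base invader projectile actor that signals hits to destructible actors it touches.
; The construction script creates the mesh's dynamic material and applies configurable scale and speed to the mesh and projectile movement, while BeginPlay tints the material with the projectile colour.
; Box overlaps send HitMessage through the IDestructible interface and destroy the projectile, ignoring actors without that interface.
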(event OnComponentBeginOverlap(Box)
  (params (OverlappedComponent :type Primitive%20Component%20Object%20Reference) (OtherActor :type Actor%20Object%20Reference) (OtherComp :type Primitive%20Component%20Object%20Reference) (OtherBodyIndex :type Integer) (bFromSweep :type Boolean) (SweepResult :type Hit%20Result%20Structure%20%28by%20ref%29))
  ;[1 1 1] Collision
  (if (Utilities|DoesObjectImplementInterface OtherActor "/Game/Interfaces/IDestructible.IDestructible_C")
    (Class|IDestructible|Hit(Message) OtherActor)
    (Actor|DestroyActor)))

(event EventBeginPlay
  ;[1 1 1] Initialise
  (Rendering|Material|SetVectorParameterValue (Variables|Default|GetProjectileMaterial) "Colour" (Variables|Default|GetProjectileColour) :!class /Script/Engine.MaterialInstanceDynamic))

(fn ConstructionScript
  (bind _projectilemovement (Variables|Default|GetProjectileMovement))
  ;[1 1 1] Instantiate
  (bind _returnvalue (Rendering|Material|CreateDynamicMaterialInstance (Variables|Default|GetProjectile) 0 0 "None" :!class /Script/Engine.PrimitiveComponent))
  (Variables|Default|SetProjectileMaterial _returnvalue)
  (Transformation|SetWorldScale3D (Variables|Default|GetProjectile) (Variables|Default|GetScale))
  (bind _output_get (Variables|/Script/Engine.ProjectileMovementComponent|SetMaxSpeed _projectilemovement (Variables|Default|GetSpeed)))
  (Variables|/Script/Engine.ProjectileMovementComponent|SetInitialSpeed _projectilemovement _output_get))