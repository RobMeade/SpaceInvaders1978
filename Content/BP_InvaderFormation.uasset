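; Invader formation actor for a Space Invaders-style game that spawns, moves and descends a grid of BP_Invader actors as one group.
; When the game mode signals game start, it attaches the spawned invaders and fits its collision box to their bounds.
; A timeline drives swept sideways movement.
; Box overlaps make it descend and reverse, except one object channel, which stops movement and triggers game over.
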(event OnComponentBeginOverlap(Collision)
  (params (OverlappedComponent :type Primitive%20Component%20Object%20Reference) (OtherActor :type Actor%20Object%20Reference) (OtherComp :type Primitive%20Component%20Object%20Reference) (OtherBodyIndex :type Integer) (bFromSweep :type Boolean) (SweepResult :type Hit%20Result%20Structure%20%28by%20ref%29))
  ;[1 1 1] Boundary Collision
  (if (Variables|Default|GetMovementEnabled)
    (if (Utilities|Enum|Equal(Enum) (Collision|GetCollisionObjectType OtherComp) "ECC_GameTraceChannel2")
      (Variables|Default|SetMovementEnabled false)
      (Default|GameOver (Variables|Default|GetGameModeReference))
      (else
        (CallFunction|Descend)
        (CallFunction|ReverseDirection)))))

(event Custom|OnGameStarted
  ;[1 1 1] Game Started
  (CallFunction|SetWaveFormation)
  (CallFunction|SpawnWave)
  (CallFunction|BeginAttack))

(event Custom|BeginAttack
  ;[1 1 1] Begin Attack
  (CallFunction|ResetInvaderFormationPosition)
  (Variables|Default|SetMovementRight true)
  (Variables|Default|SetMovementEnabled true)
  (CallFunction|Move))

(event Custom|Move
  ;[1 1 1] Movement
  (bind _alpha (Timeline|Movement PlayFromStart)
    (:Update
      (if (Variables|Default|GetMovementEnabled)
        (CallFunction|SetInvaderFormationPosition _alpha)
        (else
          (CallFunction|Stop))))))

(event Custom|Descend
  ;[1 1 1] Descend
  (bind _descentlocation (CallFunction|GetDescentPosition))
  (Transformation|SetActorLocation _descentlocation true false))

(event Custom|Stop
  ;[1 1 1] Movement
  (bind _alpha (Timeline|Movement Stop)
    (:Update
      (if (Variables|Default|GetMovementEnabled)
        (CallFunction|SetInvaderFormationPosition _alpha)
        (else
          (CallFunction|Stop))))))

(event Custom|ReverseDirection
  ;[1 1 1] Reverse Direction
  (Variables|Default|SetMovementRight (not (Variables|Default|GetMovementRight))))

(event EventBeginPlay
  ;[1 1 1] Initialise
  (CallFunction|SetReferences)
  (CallFunction|BindEvents))

(fn ConstructionScript)

(fn SetWaveFormation
  ;[1 1 1] Set Wave Formation
  (Variables|Default|SetRows 5)
  (Variables|Default|SetColumns 11))

(fn SpawnWave
  (for _index (range 0 (- (Variables|Default|GetRows) 1))
    (for _index_2 (range 0 (- (Variables|Default|GetColumns) 1))
      (bind _invader (CallFunction|SpawnInvader))
      (CallFunction|SetSpawnedInvaderPosition _invader _index_2 _index)
      (Transformation|AttachActorToActor _invader self "None" "KeepRelative" "KeepRelative" "KeepRelative" true)
      (CallFunction|UpdateCollisionVolumeExtentsandPosition))))

(fn SpawnInvader
  ;[1 1 1] Spawn Invader
  (bind _returnvalue (Game|SpawnActorfromClass "/Game/BP_Invader.BP_Invader_C" (Transformation|GetActorTransform) "AlwaysSpawn" 0 0))
  (LocalVariables|SetSpawnedInvader _returnvalue)
  (Utilities|FlowControl|Sequence
    (:then_0
      (Utilities|FlowControl|DoOnce false
        (:Completed
          (Variables|Default|SetSpawnPositionOffset (Components|Box|GetUnscaledBoxExtent (Variables|/Game/BP_Invader.BP_Invader_C|GetCollision (LocalVariables|GetSpawnedInvader)))))))
    (:then_1
      (Utilities|Array|Add (Variables|Default|GetInvaders) (LocalVariables|GetSpawnedInvader))
      (return (LocalVariables|GetSpawnedInvader)))))

(fn SetSpawnedInvaderPosition
  (params (Invader :type BP%20Invader%20Object%20Reference) (Column :type Integer) (Row :type Integer))
  ;[1 1 1] Set Invader Position
  (Transformation|SetActorTransform Invader (Math|Transform|MakeTransform (* (Math|Vector|MakeVector (* Column (.x (Variables|Default|GetSpawnPositionOffset))) 0.0 (* (* Row (.z (Variables|Default|GetSpawnPositionOffset))) -1.0)) 2) "0, 0, 0" "1,1.000000,1"))
  (return))

(fn UpdateCollisionVolumeExtentsandPosition
  ;[1 1 1] Update Collision Volume Extents and Positions
  (bind (_center _boxextent) (Collision|GetActorArrayBounds (Variables|Default|GetInvaders)))
  (Components|Box|SetBoxExtent (Variables|Default|GetCollision) _boxextent true)
  (Transformation|SetWorldLocation (Variables|Default|GetCollision) _center false true))

(fn SetReferences
  ;[1 1 1] Set References
  (bind _assi_game_mode (Utilities|Casting|CastToSI_GameMode (Game|GetGameMode)))
  (Variables|Default|SetGameModeReference _assi_game_mode))

(fn BindEvents
  ;[1 1 1] Bind Events
  (EventDispatchers|BindEventtoOnGameStarted (Variables|Default|GetGameModeReference) (EventDispatchers|CreateEvent :!event Custom|OnGameStarted)))

(fn ResetInvaderFormationPosition
  ;[1 1 1] Reset Invader Formation Position
  (Transformation|SetActorLocation (Variables|/Game/SI_GameMode.SI_GameMode_C|GetInvaderFormationSpawnLocation (Variables|Default|GetGameModeReference)) false false))

(fn GetDescentPosition
  (bind _returnvalue (Transformation|GetActorLocation))
  ;[1 1 1] Get Descent Position
  (return (Math|Vector|MakeVector (.x _returnvalue) 0.0 (- (.z _returnvalue) (* (.z (Variables|Default|GetSpawnPositionOffset)) (Variables|Default|GetDescentMultiplier))))))

(fn SetInvaderFormationPosition
  (params (Alpha :type Float%20%28single-precision%29))
  ;[1 1 1] Set Invader Formation Position
  (Transformation|SetActorLocation (+ (Transformation|GetActorLocation) (* (Math|Vector|MakeVector (* (Variables|Default|GetMovementSpeed) (Math|Float|SelectFloat 1.0 -1.0 (Variables|Default|GetMovementRight))) 0.0 0.0) Alpha)) true false))